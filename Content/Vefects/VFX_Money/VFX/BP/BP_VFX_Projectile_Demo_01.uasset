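; BP_VFX_Projectile_Demo_01 is a demo actor in the VFX_Money pack that displays a configurable Niagara effect, named as a projectile.
; The construction script assigns the chosen NiagaraSystem to the NS component, resetting override parameters, and shifts it by NSOffset.
; A timeline meant to lerp the Transform component's relative rotation between RotMin and RotMax exists, but nothing triggers it.
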(fn ConstructionScript
  (bind _ns (Variables|Default|GetNS))
  (Class|NiagaraComponent|SetAsset _ns (Variables|Default|GetNiagara_System) true)
  (Transformation|AddLocalOffset _ns (Variables|Default|GetNS_Offset) false false))